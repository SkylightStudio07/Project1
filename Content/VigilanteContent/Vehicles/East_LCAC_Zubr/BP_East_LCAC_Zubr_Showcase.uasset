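; Showcase Blueprint of the East LCAC Zubr hovercraft that exposes its features to interactive demo controls.
; Generic slider, twin-slider and checkbox events forward values to vehicle setters for turret aim, weapon fire, propeller speeds, deflation, damage and lights.
; A button event swaps ground and water environments by asynchronously streaming one sublevel in and the other out.
; The construction script only runs the parent's setup.
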(event EventSetTwinSliderVariable3
  (params (bFirstSlider? :type Boolean) (NewFirstValue :type Float%20%28single-precision%29) (NewSecondValue :type Float%20%28single-precision%29))
  ;[1 1 1] Maps twin slider controls to vehicle properties
  (CallFunction|SetPressurePropellersSpeed NewFirstValue NewSecondValue))

(event EventSetTwinSliderVariable0
  (params (bFirstSlider? :type Boolean) (NewFirstValue :type Float%20%28single-precision%29) (NewSecondValue :type Float%20%28single-precision%29))
  ;[1 1 1] Maps twin slider controls to vehicle properties
  (CallFunction|SetCannonHorizontalAngle NewFirstValue NewSecondValue))

(event EventSetCheckboxVariable0
  (params (NewState :type Boolean))
  ;[1 1 1] Maps checkbox controls to vehicle properties
  (CallFunction|SetShowDamaged NewState))

(event EventSetTwinSliderVariable1
  (params (bFirstSlider? :type Boolean) (NewFirstValue :type Float%20%28single-precision%29) (NewSecondValue :type Float%20%28single-precision%29))
  ;[1 1 1] Maps twin slider controls to vehicle properties
  (CallFunction|SetCannonElevationAngle NewFirstValue NewSecondValue))

(event EventSetTwinSliderVariable2
  (params (bFirstSlider? :type Boolean) (NewFirstValue :type Float%20%28single-precision%29) (NewSecondValue :type Float%20%28single-precision%29))
  ;[1 1 1] Maps twin slider controls to vehicle properties
  (CallFunction|SetRocketHorizontalAngle NewFirstValue NewSecondValue))

(event EventSetCheckboxVariable2
  (params (NewState :type Boolean))
  ;[1 1 1] Maps checkbox controls to vehicle properties
  (CallFunction|SetMissileLauncherFireState NewState))

(event EventSetSliderVariable0
  (params (NewValue :type Float%20%28single-precision%29))
  ;[1 1 1] Maps slider controls to vehicle properties
  (CallFunction|SetMainPropellersSpeed NewValue))

(event EventSetCheckboxVariable1
  (params (NewState :type Boolean))
  ;[1 1 1] Maps checkbox controls to vehicle properties
  (CallFunction|SetCannonFireState NewState))

(event EventSetSliderVariable1
  (params (NewValue :type Float%20%28single-precision%29))
  ;[1 1 1] Maps slider controls to vehicle properties
  (CallFunction|SetDeflation NewValue))

(event EventSetSliderVariable2
  (params (NewValue :type Float%20%28single-precision%29))
  ;[1 1 1] Maps slider controls to vehicle properties
  (CallFunction|SetLightsEmissivity NewValue))

(event EventSetButtonsVariable0
  (params (NewIndex :type Integer))
  ;[1 1 1] Switching ground and water sublevel
  (if (== NewIndex 0)
    (Class|GameplayStatics|LoadStreamLevelbySoftObjectPtr (Variables|Default|GetWaterLevel) true false)
    (Class|GameplayStatics|UnloadStreamLevelbySoftObjectPtr (Variables|Default|GetGroundLevel) false)
    (else
      (Class|GameplayStatics|LoadStreamLevelbySoftObjectPtr (Variables|Default|GetGroundLevel) true false)
      (Class|GameplayStatics|UnloadStreamLevelbySoftObjectPtr (Variables|Default|GetWaterLevel) false))))

(fn ConstructionScript
  (|CallParentFunction))